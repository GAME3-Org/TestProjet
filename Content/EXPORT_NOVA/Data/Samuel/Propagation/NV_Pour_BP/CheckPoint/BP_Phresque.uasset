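; Fresco (fresque) actor that animates a material propagation effect from an origin point, heavy with test and debug code.
; ActiveFresque maps a temporary marker between corner markers into origin X/Y parameters on the dynamic material, then repositions test objects.
; A timeline drives TestScalar while overwriting that origin with PointImpact's offset from a test cube, and clears IsActivate when finished.
; Box overlap with BP_NovaPlayer only prints debug text.
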(event OnComponentBeginOverlap(BoxDeFresque)
  (params (OverlappedComponent :type Primitive%20Component%20Object%20Reference) (OtherActor :type Actor%20Object%20Reference) (OtherComp :type Primitive%20Component%20Object%20Reference) (OtherBodyIndex :type Integer) (bFromSweep :type Boolean) (SweepResult :type Hit%20Result%20Structure%20%28by%20ref%29))
  (bind _asbp_nova_player (Utilities|Casting|CastToBP_NovaPlayer OtherActor))
  (Development|PrintString "TUEZ MOI !!" true true "(R=1.000000,G=0.643350,B=0.000000,A=1.000000)"))

(event EventBeginPlay
  ;[0 0.8793 1 1 34] BEGIN PLAY
  (Variables|Default|SetLAST_POINT_AFTER_TRACE (Transformation|GetWorldLocation (Variables|Default|GetTempPos))))

(event Collision|EventActorBeginOverlap
  (params (OtherActor :type Actor%20Object%20Reference)))

(event EventTick
  (params (DeltaSeconds :type Float%20%28single-precision%29)))

(event EventActiveFresque
  (bind _origin (Variables|Default|GetOrigin))
  (bind _temppos (Variables|Default|GetTempPos))
  (bind _last_point_after_trace (Variables|Default|GetLAST_POINT_AFTER_TRACE))
  (bind _point_impact (Variables|Default|GetPoint_Impact))
  (bind _fresquedynamicmaterialinstance (Variables|Default|GetFresqueDynamicMaterialInstance))
  (bind _testcubemesh (Variables|Default|GetTestCubeMesh))
  (bind _testcubemesh_2 (Variables|Default|GetTestCubeMesh))
  (bind _last_point_after_trace_2 (Variables|Default|GetLAST_POINT_AFTER_TRACE))
  (bind _testcubemesh_3 (Variables|Default|GetTestCubeMesh))
  (bind _returnvalue (Transformation|GetWorldLocation _testcubemesh_2))
  (bind _returnvalue_2 (Transformation|GetWorldLocation _origin))
  (bind _returnvalue_3 (Transformation|GetWorldLocation _temppos))
  (bind _returnvalue_4 (Transformation|GetWorldLocation _testcubemesh))
  (bind _returnvalue_5 (Transformation|GetWorldLocation _testcubemesh_3))
  (bind (_x _y _z) (Math|Vector|BreakVector _returnvalue_2))
  (bind _returnvalue_6 (- _point_impact _returnvalue))
  ;[0.002336 1 0.1743] Set Value X Y
  (Variables|Default|SetX_Value_A_Mettre_Pour_Origin_X (Math|Float|MapRangeClamped (.y _returnvalue_3) _y (.y (Transformation|GetWorldLocation (Variables|Default|GetMaxRight))) 0.0 0.5))
  (Variables|Default|SetY_Value_A_Mettre_Pour_Origin_Y (Math|Float|MapRangeClamped (.z _returnvalue_3) (.z (Transformation|GetWorldLocation (Variables|Default|GetMaxUp))) _z 0.0 0.5))
  ;[0 1 0.02523 1 30] Recup Valeurs TemPos en X en Y en Z
  ; Set Valeurs TemPos en X en Y en Z (avec NV_TemPos_XYZ)
  (Variables|Default|SetNV_TemPos_X (- (.x _last_point_after_trace) (.x _returnvalue_4)))
  (Variables|Default|SetNV_TemPos_Y (- (.y _last_point_after_trace) (.y _returnvalue_4)))
  (Variables|Default|SetNV_TemPos_Z (- (.z _last_point_after_trace) (.z _returnvalue_4)))
  ;[0 1 0.07378 1 34] Set World Location de Cube et TemPos (avec NV_TemPos_XYZ)
  (Transformation|SetWorldLocation (Variables|Default|GetTemPosObjet) (Math|Vector|MakeVector (Variables|Default|GetNV_TemPos_X) (Variables|Default|GetNV_TemPos_Y) (Variables|Default|GetNV_TemPos_Z)) false false)
  ;[0 1 0.0244 1 34] Verif Print Append Coordonees X & Y
  (Development|PrintString "Coordonnes_dephreseque")
  ;;[1 0 0.08355] Print X & Y
  (Development|PrintString (Utilities|String|Append (Utilities|String|ToString(Float) (Variables|Default|GetX_Value_A_Mettre_Pour_Origin_X)) (Utilities|String|ToString(Float) (Variables|Default|GetY_Value_A_Mettre_Pour_Origin_Y))) true true "(R=1.000000,G=0.000000,B=0.165000,A=1.000000)")
  ;[0.8003 0.3401 1] Correspond au Point d'Origine Pour la Propagation (Set le X et le Y de ce point)
  (Rendering|Material|SetScalarParameterValue (Variables|Default|GetFresqueDynamicMaterialInstance) "Position_Origin_X" (Variables|Default|GetX_Value_A_Mettre_Pour_Origin_X) :!class /Script/Engine.MaterialInstanceDynamic)
  (Rendering|Material|SetScalarParameterValue (Variables|Default|GetFresqueDynamicMaterialInstance) "Position_Origin_Y" (Variables|Default|GetY_Value_A_Mettre_Pour_Origin_Y) :!class /Script/Engine.MaterialInstanceDynamic)
  ;[0.4948 0.3776 0 1 34] Timeline
  (bind _newtrack_0 (Timeline|Timeline PlayFromStart)
    (:Update
      ;[0 1 0.7853 1 146] FF
      (Rendering|Debug|DrawDebugPoint (Transformation|GetWorldLocation (Variables|Default|GetTestCubeMesh)) 5.0 "(R=1.000000,G=0.000000,B=0.360840,A=1.000000)" 5.0)
      (Utilities|FlowControl|Sequence
        (:then_0
          (Rendering|Debug|DrawDebugPoint (Variables|Default|GetPoint_Impact) 1.0 "(R=0.509094,G=1.000000,B=0.000000,A=1.000000)" 5.0)
          (Rendering|Debug|DrawDebugPoint (Transformation|GetWorldLocation (Variables|Default|GetTestCubeMesh)) 1.0 "(R=1.000000,G=0.029105,B=0.000000,A=1.000000)" 5.0)
          ;[1 0.8901 0 1 58] SET ORIGIN X Y Point de propagation
          (Rendering|Material|SetScalarParameterValue _fresquedynamicmaterialinstance "Position_Origin_X" (.x _returnvalue_6) :!class /Script/Engine.MaterialInstanceDynamic)
          (Rendering|Material|SetScalarParameterValue _fresquedynamicmaterialinstance "Position_Origin_Y" (.y _returnvalue_6) :!class /Script/Engine.MaterialInstanceDynamic)
          ;[0 0.1234 1 1 58] Print X & Y
          (Development|PrintString "X:" true true "(R=1.000000,G=0.000000,B=0.532814,A=1.000000)" 8.0)
          (Development|PrintString (Utilities|String|ToString(Float) (Variables|Default|GetX_Value_A_Mettre_Pour_Origin_X)) true true "(R=1.000000,G=0.000000,B=0.895769,A=1.000000)" 8.0)
          (Development|PrintString "Y:" true true "(R=0.000000,G=0.660000,B=1.000000,A=1.000000)" 8.0)
          (Development|PrintString (Utilities|String|ToString(Float) (Variables|Default|GetY_Value_A_Mettre_Pour_Origin_Y)) true true "(R=0.000000,G=0.660000,B=1.000000,A=1.000000)" 8.0)
          ;[0.5654 1 0.6811 1 66] RESET CUBE A LA FIN
          ; ET EGALEMENT TemPos
          (Transformation|SetWorldLocation (Variables|Default|GetTemPosObjet) (Math|Vector|MakeVector (- (.x _last_point_after_trace_2) (.x _returnvalue_5)) (- (.y _last_point_after_trace_2) (.y _returnvalue_5)) (- (.z _last_point_after_trace_2) (.z _returnvalue_5))) false false)
          ;[0.6469 0.3534 1] Correspond A Time
          (Rendering|Material|SetScalarParameterValue (Variables|Default|GetFresqueDynamicMaterialInstance) "TestScalar" _newtrack_0 :!class /Script/Engine.MaterialInstanceDynamic)
          ;[0.6586 0 1] -----TEST-----CubeOrange
          (Transformation|SetWorldLocation (Variables|Default|GetTemPosObjetOrange) (Math|Vector|MakeVector (Variables|Default|GetNV_TemPos_X) (Variables|Default|GetNV_TemPos_Y) (Variables|Default|GetNV_TemPos_Z)) false false))
        (:then_2
          (bind _asbp_nova_player (Utilities|Casting|CastToBP_NovaPlayer (stale OnComponentBeginOverlap(BoxDeFresque) OtherActor)))
          (Development|PrintString "TUEZ MOI !!" true true "(R=1.000000,G=0.643350,B=0.000000,A=1.000000)"))))
    (:Finished
      ;;[1 0.06918 0.1489] Boolean
      (Variables|Default|SetbIsActivate false))))

(fn ConstructionScript)
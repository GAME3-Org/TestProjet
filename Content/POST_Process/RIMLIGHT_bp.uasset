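; RIMLIGHT_bp is a rim light control Blueprint that applies lighting settings to the materials on its PaimonTest component.
; The Construction Script creates a dynamic material instance for each slot and writes the angle, spread, intensity, hardness and color variables into its RimLight parameters.
; Each slot then receives a SetMaterial call with the loop's array element rather than the created instance reference.
; The event graph holds no active logic.
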(event EventBeginPlay)

(event Collision|EventActorBeginOverlap
  (params (OtherActor :type Actor%20Object%20Reference)))

(event EventTick
  (params (DeltaSeconds :type Float%20%28single-precision%29)))

(fn ConstructionScript
  (bind _paimontest (Variables|Default|GetPaimonTest))
  (for (_array_element _array_index) (Rendering|Material|GetMaterials _paimontest)
    (bind _returnvalue (Rendering|Material|CreateDynamicMaterialInstance _paimontest _array_index _array_element "None" :!class /Script/Engine.PrimitiveComponent))
    (Rendering|Material|SetScalarParameterValue _returnvalue "RimLight_Angle" (Variables|Default|GetRimLight_Angle) :!class /Script/Engine.MaterialInstanceDynamic)
    (Rendering|Material|SetScalarParameterValue _returnvalue "RimLight_Spread" (Variables|Default|GetRimLight_Spread) :!class /Script/Engine.MaterialInstanceDynamic)
    (Rendering|Material|SetScalarParameterValue _returnvalue "RimLight_Intensity" (Variables|Default|GetRimLight_Intensity) :!class /Script/Engine.MaterialInstanceDynamic)
    (Rendering|Material|SetScalarParameterValue _returnvalue "RimLight_Hardness" (Variables|Default|GetRimLight_Hardness) :!class /Script/Engine.MaterialInstanceDynamic)
    (Rendering|Material|SetVectorParameterValue _returnvalue "RimLight_Color" (Math|Conversions|ToLinearColor(Color) (Variables|Default|GetRimLight_Color)) :!class /Script/Engine.MaterialInstanceDynamic)
    (Rendering|Material|SetMaterial _paimontest _array_index _array_element)))
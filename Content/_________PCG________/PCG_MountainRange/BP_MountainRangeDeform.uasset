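; BP_MountainRangeDeform is an actor that deforms landscape height through a LandscapeTexturePatch, as part of the PCG mountain range setup.
; Its construction script feeds the configured texture and blend mode into the patch as a texture-asset height source.
; The height encoding scale is random between a min and max, so it re-rolls whenever construction reruns.
; The event graph holds no active logic.
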(event EventBeginPlay)

(event Collision|EventActorBeginOverlap
  (params (OtherActor :type Actor%20Object%20Reference)))

(event EventTick
  (params (DeltaSeconds :type Float%20%28single-precision%29)))

(fn ConstructionScript
  (bind _landscapetexturepatch (Variables|Default|GetLandscapeTexturePatch))
  (bind _landscapetexturepatch_2 (Variables|Default|GetLandscapeTexturePatch))
  (Class|LandscapeTexturePatch|SetHeightSourceMode _landscapetexturepatch "TextureAsset")
  (Class|LandscapeTexturePatch|SetBlendMode _landscapetexturepatch (Variables|Default|GetBlend%20Mode))
  (Class|LandscapeTexturePatch|SetHeightTextureAsset _landscapetexturepatch_2 (Variables|Default|GetTexture))
  (Class|LandscapeTexturePatch|SetHeightEncodingSettings _landscapetexturepatch_2 (Utilities|Struct|MakeLandscapeTexturePatchEncodingSettings 0.0 (Math|Random|RandomFloatinRange (Variables|Default|GetHeightScaleMin) (Variables|Default|GetHeightScaleMax)))))
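; BP_BlockTestBuilder is a generated dynamic mesh actor that builds a wall block with a rectangular opening cut into it.
; On mesh rebuild, Geometry Script appends a box from WallSize, then builds a cutter from an upright rectangle extruded along Y by the CutoutSize depth.
; A boolean subtract at CutoutLocation carves the cutter out of the wall.
; BeginPlay, Tick and the construction script are empty.
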(event EventBeginPlay)

(event Collision|EventActorBeginOverlap
  (params (OtherActor :type Actor%20Object%20Reference)))

(event EventTick
  (params (DeltaSeconds :type Float%20%28single-precision%29)))

(event Events|EventOnRebuildGeneratedMesh
  (params (TargetMesh :type Dynamic%20Mesh%20Object%20Reference))
  (bind _wallsize (Variables|Default|GetWallSize))
  (bind _cutoutsize (Variables|Default|GetCutoutSize))
  (Variables|Default|SetDynamic%20Mesh TargetMesh)
  (Utilities|FlowControl|Sequence
    (:then_0
      ;[1 1 1] Create Wall
      (Class|GeometryScriptLibraryMeshPrimitiveFunctions|AppendBox :TargetMesh (Variables|Default|GetDynamic%20Mesh) :DimensionX (.x _wallsize) :DimensionY (.y _wallsize) :DimensionZ (.z _wallsize) :Debug 0))
    (:then_1
      ;[1 1 1] create cutout
      (bind _returnvalue (DynamicMeshActor|AllocateComputeMesh))
      (bind _returnvalue_2 (Class|GeometryScriptLibraryMeshPrimitiveFunctions|AppendRectangleXY :TargetMesh _returnvalue :Transform (Math|Transform|MakeTransform "0, 0, 0" "0.000000,0.000000,90.000000" "1.000000,1.000000,1.000000") :DimensionX (.x _cutoutsize) :DimensionY (.z _cutoutsize) :Debug 0))
      (Variables|Default|SetCutout%20Mesh _returnvalue_2))
    (:then_2
      ;[1 1 1] extrude cutout
      (bind _returnvalue_3 (Class|GeometryScriptLibraryMeshModelingFunctions|ApplyMeshExtrudeCompatibility5p0 (Variables|Default|GetCutout%20Mesh) (Utilities|Struct|MakeGeometryScriptMeshExtrudeOptions (.y (Variables|Default|GetCutoutSize)) "0.000000,1.000000,0.000000" 1.0 true) 0))
      (Variables|Default|SetCutout%20Mesh _returnvalue_3))
    (:then_3
      ;[1 1 1] apply cutout boolean
      (bind _returnvalue_4 (GeometryScript|Booleans|ApplyMeshBoolean :TargetMesh (Variables|Default|GetDynamic%20Mesh) :ToolMesh (Variables|Default|GetCutout%20Mesh) :ToolTransform (Math|Transform|MakeTransform (Variables|Default|GetCutoutLocation) "0, 0, 0" "1.000000,1.000000,1.000000") :Operation "Subtract" :Debug 0))
      (Variables|Default|SetDynamic%20Mesh _returnvalue_4))))

(fn ConstructionScript)
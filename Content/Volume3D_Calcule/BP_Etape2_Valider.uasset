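; Generated dynamic mesh actor that serves as a volume calculation test step, printing measurements of a static mesh on screen at play start.
; BeginPlay resets its dynamic mesh, copies Sphere1 into it and reads surface area and volume through Geometry Script.
; It also prints both values divided by the LOD 0 triangle count of StaticMeshRecup, a separate reference from Sphere1.
; Mesh splitting, wall cutout boolean and other experiments are left unconnected.
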(event EventBeginPlay
  (bind _staticmeshrecup (Variables|Default|GetStaticMeshRecup))
  (bind _returnvalue (Class|StaticMesh|GetNumTriangles _staticmeshrecup))
  ;[1 1 1] Etape2
  (bind _returnvalue_2 (DynamicMeshComponent|GetDynamicMesh (Variables|DynamicMeshActor|GetDynamicMeshComponent)))
  (bind _returnvalue_3 (DynamicMesh|Reset _returnvalue_2))
  (bind _returnvalue_4 (GeometryScript|StaticMesh|CopyMeshFromStaticMesh :FromStaticMeshAsset "/Game/Volume3D_Calcule/Sphere1.Sphere1" :ToDynamicMesh _returnvalue_3 :Debug 0)
    (:Failure
      (Development|PrintString "failure"))
    (:Success
      (Utilities|FlowControl|Sequence
        (:then_0
          (Development|PrintString "surface area" true true "(R=0.000000,G=1.000000,B=0.339822,A=1.000000)" 1e+01)
          (Development|PrintString (Utilities|String|ToString(Float) (.SurfaceArea (Class|GeometryScriptLibraryMeshQueryFunctions|GetMeshVolumeArea _returnvalue_4))) true true "(R=0.000000,G=1.000000,B=0.360225,A=1.000000)" 1e+01)
          (Development|PrintString "volume" true true "(R=0.500000,G=0.000000,B=1.000000,A=1.000000)" 1e+01)
          (Development|PrintString (Utilities|String|ToString(Float) (.Volume (Class|GeometryScriptLibraryMeshQueryFunctions|GetMeshVolumeArea _returnvalue_4))) true true "(R=0.277748,G=0.000000,B=1.000000,A=1.000000)" 1e+01))
        (:then_1
          (Development|PrintString "surface area divid tris" true true "(R=1.000000,G=0.573006,B=0.000000,A=1.000000)" 1e+01)
          (Development|PrintString (Utilities|String|ToString(Float) (/ (.SurfaceArea (Class|GeometryScriptLibraryMeshQueryFunctions|GetMeshVolumeArea _returnvalue_4)) _returnvalue)) true true "(R=1.000000,G=0.615952,B=0.000000,A=1.000000)" 1e+01)
          (Development|PrintString "volume divid tris" true true "(R=1.000000,G=0.864047,B=0.000000,A=1.000000)" 1e+01)
          (Development|PrintString (Utilities|String|ToString(Float) (/ (.Volume (Class|GeometryScriptLibraryMeshQueryFunctions|GetMeshVolumeArea _returnvalue_4)) _returnvalue)) true true "(R=1.000000,G=0.800593,B=0.000000,A=1.000000)" 1e+01))))))

(event Collision|EventActorBeginOverlap
  (params (OtherActor :type Actor%20Object%20Reference)))

(event EventTick
  (params (DeltaSeconds :type Float%20%28single-precision%29)))

(event Events|EventOnRebuildGeneratedMesh
  (params (TargetMesh :type Dynamic%20Mesh%20Object%20Reference)))

(fn ConstructionScript)
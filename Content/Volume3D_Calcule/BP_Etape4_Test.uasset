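; Test GeneratedDynamicMeshActor Blueprint that measures a static mesh's geometry and prints the results as on-screen debug text.
; On BeginPlay it reads StaticMeshRecup's LOD counts and triangle count, then copies it into its DynamicMeshComponent through Geometry Script.
; It stores the copy's surface area and volume and prints both, also divided by triangle count.
; Unconnected experiments remain for volume-tolerance checks, LOD edits, mesh splitting and boolean wall cutouts.
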(event EventBeginPlay
  (bind _staticmeshrecup (Variables|Default|GetStaticMeshRecup))
  (bind _staticmeshrecup_2 (Variables|Default|GetStaticMeshRecup))
  (bind _returnvalue (Class|StaticMesh|GetNumTriangles _staticmeshrecup))
  (bind _returnvalue_2 (Class|StaticMesh|GetNumTriangles _staticmeshrecup_2))
  (Utilities|FlowControl|Sequence
    (:then_0
      (bind _returnvalue_3 (Class|GeometryScriptLibraryStaticMeshFunctions|GetNumStaticMeshLODsOfType (Variables|Default|GetStaticMeshRecup) "MaxAvailable"))
      (Development|PrintString (Utilities|String|ToString(Integer) _returnvalue_3) true true "(R=0.858357,G=1.000000,B=0.000000,A=1.000000)"))
    (:then_2
      (Development|PrintString "NUmbre de triangles:")
      (Development|PrintString (Utilities|String|ToString(Integer) _returnvalue_2))
      (Variables|Default|SetNumberTrianglesOfSM _returnvalue_2))
    (:then_3
      (bind _returnvalue_4 (DynamicMeshComponent|GetDynamicMesh (Variables|DynamicMeshActor|GetDynamicMeshComponent)))
      (bind _returnvalue_5 (DynamicMesh|Reset _returnvalue_4))
      (bind _returnvalue_6 (GeometryScript|StaticMesh|CopyMeshFromStaticMesh :FromStaticMeshAsset (Variables|Default|GetStaticMeshRecup) :ToDynamicMesh _returnvalue_5 :Debug 0)
        (:Failure
          (Development|PrintString "failure"))
        (:Success
          (Utilities|FlowControl|Sequence
            (:then_0
              (Development|PrintString "surface area" true true "(R=0.000000,G=1.000000,B=0.339822,A=1.000000)" 1e+01)
              (Development|PrintString (Utilities|String|ToString(Float) (.SurfaceArea (Class|GeometryScriptLibraryMeshQueryFunctions|GetMeshVolumeArea _returnvalue_6))) true true "(R=0.000000,G=1.000000,B=0.360225,A=1.000000)" 1e+01)
              (Development|PrintString "volume" true true "(R=0.500000,G=0.000000,B=1.000000,A=1.000000)" 1e+01)
              (Development|PrintString (Utilities|String|ToString(Float) (.Volume (Class|GeometryScriptLibraryMeshQueryFunctions|GetMeshVolumeArea _returnvalue_6))) true true "(R=0.277748,G=0.000000,B=1.000000,A=1.000000)" 1e+01)
              (Variables|Default|SetSurfaceAreaOfDynamesh (.SurfaceArea (Class|GeometryScriptLibraryMeshQueryFunctions|GetMeshVolumeArea _returnvalue_6)))
              (Variables|Default|SetVolumeOfDynamesh (.Volume (Class|GeometryScriptLibraryMeshQueryFunctions|GetMeshVolumeArea _returnvalue_6))))
            (:then_1
              (Development|PrintString "surface area divid tris" true true "(R=1.000000,G=0.573006,B=0.000000,A=1.000000)" 1e+01)
              (Development|PrintString (Utilities|String|ToString(Float) (/ (.SurfaceArea (Class|GeometryScriptLibraryMeshQueryFunctions|GetMeshVolumeArea _returnvalue_6)) _returnvalue)) true true "(R=1.000000,G=0.615952,B=0.000000,A=1.000000)" 1e+01)
              (Development|PrintString "volume divid tris" true true "(R=1.000000,G=0.864047,B=0.000000,A=1.000000)" 1e+01)
              (Development|PrintString (Utilities|String|ToString(Float) (/ (.Volume (Class|GeometryScriptLibraryMeshQueryFunctions|GetMeshVolumeArea _returnvalue_6)) _returnvalue)) true true "(R=1.000000,G=0.800593,B=0.000000,A=1.000000)" 1e+01))))))
    (:then_4
      (bind _returnvalue_7 (Class|GeometryScriptLibraryStaticMeshFunctions|GetNumStaticMeshLODsOfType (Variables|Default|GetStaticMeshRecup) "SourceModel"))
      (Development|PrintString (Utilities|String|ToString(Integer) _returnvalue_7) true true "(R=1.000000,G=0.000000,B=0.773749,A=1.000000)" 12.0))))

(event Collision|EventActorBeginOverlap
  (params (OtherActor :type Actor%20Object%20Reference)))

(event EventTick
  (params (DeltaSeconds :type Float%20%28single-precision%29)))

(event Events|EventOnRebuildGeneratedMesh
  (params (TargetMesh :type Dynamic%20Mesh%20Object%20Reference)))

(fn ConstructionScript)
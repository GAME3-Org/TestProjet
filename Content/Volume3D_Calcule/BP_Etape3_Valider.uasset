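; Geometry Script test actor for computing 3D mesh volume; at runtime it only prints the source-model LOD count of StaticMeshRecup on BeginPlay.
; Disconnected experiments copy static meshes into dynamic meshes to print surface area, volume and per-triangle ratios.
; Other unwired chains split selected mesh assets by component and cut an extruded opening from a box wall with a boolean subtract.
; The mesh rebuild event and construction script are empty.
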(event EventBeginPlay
  (bind _returnvalue (Class|GeometryScriptLibraryStaticMeshFunctions|GetNumStaticMeshLODsOfType (Variables|Default|GetStaticMeshRecup) "SourceModel"))
  (Development|PrintString (Utilities|String|ToString(Integer) _returnvalue) true true "(R=1.000000,G=0.000000,B=0.773749,A=1.000000)" 12.0))

(event Collision|EventActorBeginOverlap
  (params (OtherActor :type Actor%20Object%20Reference)))

(event EventTick
  (params (DeltaSeconds :type Float%20%28single-precision%29)))

(event Events|EventOnRebuildGeneratedMesh
  (params (TargetMesh :type Dynamic%20Mesh%20Object%20Reference)))

(fn ConstructionScript)
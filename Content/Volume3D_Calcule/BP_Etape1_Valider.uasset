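; Generated dynamic mesh actor that serves as a debug test for reading triangle counts, apparently a first validation step for 3D volume calculation.
; On BeginPlay it prints the LOD 0 triangle count of StaticMeshRecup.
; On mesh rebuild it stores the target as DynamicMesh and prints its triangle count.
; Unconnected Geometry Script leftovers, including a wall with a boolean-subtracted extruded cutout, never run.
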(event EventBeginPlay
  (Development|PrintString "NUmbre de triangles:")
  (Development|PrintString (Utilities|String|ToString(Integer) (Class|StaticMesh|GetNumTriangles (Variables|Default|GetStaticMeshRecup)))))

(event Collision|EventActorBeginOverlap
  (params (OtherActor :type Actor%20Object%20Reference)))

(event EventTick
  (params (DeltaSeconds :type Float%20%28single-precision%29)))

(event Events|EventOnRebuildGeneratedMesh
  (params (TargetMesh :type Dynamic%20Mesh%20Object%20Reference))
  (bind _output_get (Variables|Default|SetDynamic%20Mesh TargetMesh))
  (Development|PrintString (Utilities|String|ToString(Integer) (Class|DynamicMesh|GetTriangleCount _output_get))))

(fn ConstructionScript)
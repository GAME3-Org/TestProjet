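; Test actor that measures the surface area and volume of a static mesh using Geometry Script.
; On BeginPlay it resets its DynamicMeshComponent's mesh, copies a sphere static mesh into it, then prints both values, or a failure message.
; The remaining graphs are disconnected experiments, including splitting selected assets by components, triangle counts, and a wall with a boolean-subtracted cutout.
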(event EventBeginPlay
  (bind _returnvalue (DynamicMeshComponent|GetDynamicMesh (Variables|DynamicMeshActor|GetDynamicMeshComponent)))
  (bind _returnvalue_2 (DynamicMesh|Reset _returnvalue))
  (bind _returnvalue_3 (GeometryScript|StaticMesh|CopyMeshFromStaticMesh :FromStaticMeshAsset "/Game/Volume3D_Calcule/Sphere1.Sphere1" :ToDynamicMesh _returnvalue_2 :Debug 0)
    (:Failure
      (Development|PrintString "failure"))
    (:Success
      (Development|PrintString "surface area")
      (Development|PrintString (Utilities|String|ToString(Float) (.SurfaceArea (Class|GeometryScriptLibraryMeshQueryFunctions|GetMeshVolumeArea _returnvalue_3))))
      (Development|PrintString "volume")
      (Development|PrintString (Utilities|String|ToString(Float) (.Volume (Class|GeometryScriptLibraryMeshQueryFunctions|GetMeshVolumeArea _returnvalue_3)))))))

(event Collision|EventActorBeginOverlap
  (params (OtherActor :type Actor%20Object%20Reference)))

(event EventTick
  (params (DeltaSeconds :type Float%20%28single-precision%29)))

(event Events|EventOnRebuildGeneratedMesh
  (params (TargetMesh :type Dynamic%20Mesh%20Object%20Reference)))

(fn ConstructionScript)
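; BP_ModularWallsContinue is a procedural level-art tool that builds a straight row of repeated modular meshes, such as wall segments.
; The Construction Script assigns MeshModule to the InstanceGroup component and derives the module length from its Y bounds.
; It then adds InstanceCount instances in local space along Y, spaced by that length so the bounds sit end to end.
; The Event Graph holds only disabled placeholder events, so there is no runtime logic.
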(event EventBeginPlay)

(event Collision|EventActorBeginOverlap
  (params (OtherActor :type Actor%20Object%20Reference)))

(event EventTick
  (params (DeltaSeconds :type Float%20%28single-precision%29)))

(fn ConstructionScript
  (Utilities|FlowControl|Sequence
    (:then_0
      (Components|StaticMesh|SetStaticMesh (Variables|Default|GetInstanceGroup) (Variables|Default|GetMeshModule)))
    (:then_1
      (LocalVariables|SetMeshLength (* (.Y (Math|Vector|BreakVector (.boxextent (StaticMesh|GetBounds (Variables|Default|GetMeshModule))))) 2.0)))
    (:then_2
      (for _index (range 0 (- (Variables|Default|GetInstanceCount) 1))
        (Components|InstancedStaticMesh|AddInstance (Variables|Default|GetInstanceGroup) (Math|Transform|MakeTransform (Math|Vector|MakeVector 0.0 (* _index (LocalVariables|GetMeshLength)) 0.0)) false)))))
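; BP_ModularWalls is a procedural level-art tool that builds a straight modular wall along local X in its construction script.
; It divides the LastInstanceEnd X distance by the wall mesh's bounds length to get a whole module count.
; It then adds instanced wall meshes at that spacing, each paired with a connector offset by ConnectorTransform.
; A stretch-to-fit scale is computed but not applied, and debug prints remain.
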(event EventBeginPlay)

(event Collision|EventActorBeginOverlap
  (params (OtherActor :type Actor%20Object%20Reference)))

(event EventTick
  (params (DeltaSeconds :type Float%20%28single-precision%29)))

(fn ConstructionScript
  (Utilities|FlowControl|Sequence
    (:then_0
      (Components|StaticMesh|SetStaticMesh (Variables|Default|GetInstanceGrpWall) (Variables|Default|GetMeshModule))
      (Components|StaticMesh|SetStaticMesh (Variables|Default|GetInstanceGrpConnector) (Variables|Default|GetMeshConnector)))
    (:then_1
      (LocalVariables|SetMeshLength (* (.X (Math|Vector|BreakVector (.boxextent (StaticMesh|GetBounds (Variables|Default|GetMeshModule))))) 2.0)))
    (:then_2
      (bind _output_get (LocalVariables|SetDistanceToEnd (Math|Float|Max(Float) (.x (Variables|Default|GetLastInstanceEnd)) 1.0)))
      (Development|PrintString (Utilities|String|ToString(Float) _output_get)))
    (:then_3
      (Development|PrintString (Utilities|String|ToString(Float) (/ (LocalVariables|GetDistanceToEnd) (LocalVariables|GetMeshLength))))
      (Variables|Default|SetInstanceCount (Math|Float|Floor (/ (LocalVariables|GetDistanceToEnd) (LocalVariables|GetMeshLength))))
      (LocalVariables|SetScaleToMatchEnd (/ (/ (LocalVariables|GetDistanceToEnd) (LocalVariables|GetMeshLength)) (Math|Conversions|ToFloat(Integer) (Math|Float|Floor (/ (LocalVariables|GetDistanceToEnd) (LocalVariables|GetMeshLength)))))))
    (:then_4
      (for _index (range 0 (- (Variables|Default|GetInstanceCount) 1))
        (Components|InstancedStaticMesh|AddInstance (Variables|Default|GetInstanceGrpWall) (Math|Transform|MakeTransform (Math|Vector|MakeVector (* _index (LocalVariables|GetMeshLength)) 0.0 0.0)) false)
        (Components|InstancedStaticMesh|AddInstance (Variables|Default|GetInstanceGrpConnector) (Math|Transform|ComposeTransforms (Math|Transform|MakeTransform (Math|Vector|MakeVector (* _index (LocalVariables|GetMeshLength)) 0.0 0.0)) (Variables|Default|GetConnectorTransform)) false)))))
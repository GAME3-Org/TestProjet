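; Procedural level-art Blueprint that builds a modular wall along local X up to an end point, with connectors and scattered decorations.
; The construction script rounds distance over mesh length to a module count and stretches modules in X to fit exactly.
; Walls and connectors are instanced meshes, while decorations are individual components randomly picked and placed from a random stream within module bounds, offset by the connector transform.
; Debug spheres mark each decoration point.
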(event EventBeginPlay)

(event Collision|EventActorBeginOverlap
  (params (OtherActor :type Actor%20Object%20Reference)))

(event EventTick
  (params (DeltaSeconds :type Float%20%28single-precision%29)))

(fn ConstructionScript
  (Utilities|FlowControl|Sequence
    (:then_0
      (CallFunction|Initialize))
    (:then_1
      (LocalVariables|SetMeshLength (CallFunction|CalcMeshLength)))
    (:then_2
      (bind _output_get (LocalVariables|SetDistanceToEnd (CallFunction|CalcDistancetoEnd)))
      (Development|PrintString (Utilities|String|ToString(Float) _output_get)))
    (:then_3
      (bind (_instance_count _scale_to_match_end) (CallFunction|CalcInstanceCountandScale (LocalVariables|GetDistanceToEnd) (LocalVariables|GetMeshLength)))
      (Variables|Default|SetInstanceCount _instance_count)
      (LocalVariables|SetScaleToMatchEnd _scale_to_match_end))
    (:then_4
      (for _index (range 0 (- (Variables|Default|GetInstanceCount) 1))
        (bind (_index_2 _transform) (CallFunction|AddModule _index (LocalVariables|GetMeshLength) (LocalVariables|GetScaleToMatchEnd)))
        (CallFunction|AddDecorations _transform _index_2)))))

(fn Initialize
  (Components|StaticMesh|SetStaticMesh (Variables|Default|GetInstanceGrpWall) (Variables|Default|GetMeshModule))
  (Components|StaticMesh|SetStaticMesh (Variables|Default|GetInstanceGrpConnector) (Variables|Default|GetMeshConnector)))

(fn CalcMeshLength
  (return (* (.X (Math|Vector|BreakVector (.boxextent (StaticMesh|GetBounds (Variables|Default|GetMeshModule))))) 2.0)))

(fn CalcDistancetoEnd
  (return (Math|Float|Max(Float) (.x (Variables|Default|GetLastInstanceEnd)) 1.0)))

(fn CalcInstanceCountandScale
  (params (TEMPO_DistanceToEnd :type Float%20%28double-precision%29) (TEMPO_MeshLength :type Float%20%28double-precision%29))
  (bind _returnvalue (/ TEMPO_DistanceToEnd TEMPO_MeshLength))
  (bind _returnvalue_2 (Math|Float|Round _returnvalue))
  (return _returnvalue_2 (/ _returnvalue (Math|Conversions|ToFloat(Integer) _returnvalue_2))))

(fn AddModule
  (params (InstanceIndex :type Integer) (TEMPO_MeshLength :type Float%20%28double-precision%29) (TEMPO_Scale%20to%20Ma :type Float%20%28double-precision%29))
  (bind _returnvalue (* InstanceIndex TEMPO_MeshLength))
  (bind _connectortransform (Variables|Default|GetConnectorTransform))
  (bind _returnvalue_2 (* _returnvalue TEMPO_Scale%20to%20Ma))
  (bind _returnvalue_3 (Math|Transform|MakeTransform (Math|Vector|MakeVector _returnvalue_2 0.0 0.0) "0, 0, 0" (Math|Vector|MakeVector TEMPO_Scale%20to%20Ma 1.0 1.0)))
  (bind _returnvalue_4 (Math|Transform|ComposeTransforms _returnvalue_3 _connectortransform))
  (Components|InstancedStaticMesh|AddInstance (Variables|Default|GetInstanceGrpWall) _returnvalue_3 false)
  (bind _returnvalue_5 (Components|InstancedStaticMesh|AddInstance (Variables|Default|GetInstanceGrpConnector) _returnvalue_4 false))
  (return _returnvalue_5 _returnvalue_4))

(fn AddDecorations
  (params (module%20transform :type Transform) (InstanceIndex :type Integer))
  (bind _decorationmeshes (Variables|Default|GetDecorationMeshes))
  (bind _output_get (LocalVariables|SetDecorationCount 9))
  (for _index (range 0 (- _output_get 1))
    (bind _local_position (CallFunction|GetRandomPointWithinModule (Variables|Default|GetMeshModule) module%20transform InstanceIndex))
    (bind _returnvalue (AddComponent|AddStaticMeshComponent false (Math|Transform|MakeTransform _local_position "0, 0, 0" "1.000000,1.000000,1.000000")))
    (Components|StaticMesh|SetStaticMesh _returnvalue (Utilities|Array|Get(acopy) _decorationmeshes (Math|Random|RandomIntegerinRangefromStream (Variables|Default|GetRandmStream) 0 (- (Utilities|Array|Length _decorationmeshes) 1))))
    (Rendering|Debug|DrawDebugSphere (Math|Transform|TransformLocation (Transformation|GetActorTransform) _local_position) 3e+01 12 "(R=1.000000,G=1.000000,B=1.000000,A=1.000000)" 0.5 2.0)))

(fn GetRandomPointWithinModule
  (params (ModuleMesh :type Static%20Mesh%20Object%20Reference) (ModuleTrandform :type Transform%20%28by%20ref%29) (InstanceIndex :type Integer))
  (bind _returnvalue (StaticMesh|GetBounds ModuleMesh))
  (Utilities|FlowControl|Sequence
    (:then_1
      ;[1 1 1] Get Random X
      (LocalVariables|SetRandomX (Math|Random|RandomFloatinRangefromStream (Variables|Default|GetRandmStream) -1.0 1.0)))
    (:then_3
      ;[1 1 1] Get Random Z
      (LocalVariables|SetRandomZ (Math|Random|RandomFloatinRangefromStream (Variables|Default|GetRandmStream) -1.0 1.0)))
    (:then_4
      (return (Math|Transform|TransformLocation ModuleTrandform (* (+ (* (Math|Vector|MakeVector (LocalVariables|GetRandomX) 0.0 (LocalVariables|GetRandomZ)) (.boxextent _returnvalue)) (.origin _returnvalue)) (.Scale (Math|Transform|BreakTransform ModuleTrandform))))))))
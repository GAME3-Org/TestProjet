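; Test actor blueprint, named for modifying an actor's static mesh, that experiments with procedural mesh creation at runtime.
; On BeginPlay, DoSomething prints a debug message, requests a dynamic mesh from a pool, calls CreateStaticMeshDescription with it and returns it to the pool.
; Unconnected leftover nodes for a generated-asset path, dynamic materials, smoothing groups and click binding never run, and the construction script is empty.
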(event Custom|Do%20Something
  (Development|PrintString "Hello")
  (bind _returnvalue (Class|DynamicMeshPool|RequestMesh (Variables|Default|GetDynamic%20Mesh%20Pool)))
  (bind _output_get (Variables|Default|SetDynamic%20Mesh _returnvalue))
  (Class|StaticMesh|CreateStaticMeshDescription _output_get)
  (Class|DynamicMeshPool|ReturnMesh (Variables|Default|GetDynamic%20Mesh%20Pool) (Variables|Default|GetDynamic%20Mesh)))

(event EventBeginPlay
  (CallFunction|DoSomething))

(event Collision|EventActorBeginOverlap
  (params (OtherActor :type Actor%20Object%20Reference)))

(event EventTick
  (params (DeltaSeconds :type Float%20%28single-precision%29)))

(fn ConstructionScript)